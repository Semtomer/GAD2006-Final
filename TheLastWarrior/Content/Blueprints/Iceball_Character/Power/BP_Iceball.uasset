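; Iceball projectile for the Iceball character, serving both thrown base attacks and strong attacks.
; BeginPlay caches game instance and player state, raising gravity for strong attacks.
; On hit, it swaps trail for impact Niagara, offset by player facing for throws or raised for strong attacks, and plays a crash sound.
; GiveEffect then once damages overlapping enemies using settings damage plus any critical bonus, and destroys itself after a delay.
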(event OnComponentHit(Collision)
  (params (HitComponent :type Primitive%20Component%20Object%20Reference) (OtherActor :type Actor%20Object%20Reference) (OtherComp :type Primitive%20Component%20Object%20Reference) (NormalImpulse :type Vector :default "0, 0, 0") (Hit :type Hit%20Result%20Structure%20%28by%20ref%29))
  (Components|Activation|Deactivate (Variables|Default|GetNS_Projectile))
  (Components|Activation|SetActive (Variables|Default|GetNS_Projectile_Hit) true false)
  (Variables|Default|SetImpactPoint (.ImpactPoint (Collision|BreakHitResult Hit)))
  ;[1 1 1] Spawns the fireball projectile according to the direction the character is looking at.
  (bind (_north _east _south _west) (Default|GivePlayerDirection (Variables|Default|GetCharRef)))
  (if _north
    (Utilities|GiveEffect (- (Variables|Default|GetImpactPoint) "-100.000000, 0,0.000000"))
    (elif _east
      (Utilities|GiveEffect (- (Variables|Default|GetImpactPoint) "0.000000,-100.000000,0.000000"))
      (elif _south
        (Utilities|GiveEffect (- (Variables|Default|GetImpactPoint) "100.000000, 0,0.000000"))
        (elif _west
          (Utilities|GiveEffect (- (Variables|Default|GetImpactPoint) "0.000000,100.000000,0.000000")))))))

(event EventBeginPlay
  (bind _asbp_game_instance (Utilities|Casting|CastToBP_GameInstance (Game|GetGameInstance)))
  (Variables|Default|SetGameInstanceRef _asbp_game_instance)
  (Class|NiagaraComponent|SetAsset (Variables|Default|GetNS_Projectile) (Variables|Default|GetProjectile) true)
  (Class|NiagaraComponent|SetAsset (Variables|Default|GetNS_Projectile_Hit) (Variables|Default|GetHit) true)
  (Components|Activation|Deactivate (Variables|Default|GetNS_Projectile_Hit))
  (bind _asbp_iceball_char (Utilities|Casting|CastToBP_Iceball_Char (Game|Player|GetPlayerPawn 0)))
  (bind _output_get (Variables|Default|SetCharRef _asbp_iceball_char))
  (Variables|Default|SetisCriticalDamageActive (Variables|/Game/Blueprints/Iceball_Character/BP_Iceball_Char.BP_Iceball_Char_C|GetisCriticalDamageActive? _output_get))
  (if (Variables|/Game/Blueprints/Iceball_Character/BP_Iceball_Char.BP_Iceball_Char_C|GetisThrowing? (Variables|Default|GetCharRef))
    (Variables|Default|SetisThrowing true)
    (else
      ;[1 1 1] For strong attack
      (Variables|/Script/Engine.ProjectileMovementComponent|SetProjectileGravityScale (Variables|Default|GetProjectileMovement) 15.0)
      (Utilities|FlowControl|Delay 0.2))))

(fn ConstructionScript)