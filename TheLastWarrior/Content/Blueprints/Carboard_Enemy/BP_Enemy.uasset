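; BP_Enemy is an AI melee enemy that runs the BT_Enemy behavior tree.
; Its attack damages overlapping actors of the Warrior, Fireball or Iceball class, chosen by the game instance's PlayerIndex.
; ModifyDamage sets a hit flag and plays a sound, while a looping timer clears the flag after a short delay.
; Death switches animation state, stops AI logic, ignores pawn collision and destroys the actor after a delay.
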(event Custom|DamageControl
  ;[1 0 0.9725] If damaged, it will run the damage animation.
  (if (Variables|Default|GetisDamage?)
    (Utilities|FlowControl|Delay 0.6)
    (if (Variables|Default|GetisDamage?)
      (Variables|Default|SetisDamage? false))))

(event Custom|AI%20Attack
  ;[1 0 0.04792] Enemy deals damage to the character within hit range of the melee attack.
  (if (Variables|Default|GetisAttack?)
    (bind _asbp_game_instance (Utilities|Casting|CastToBP_GameInstance (Game|GetGameInstance)))
    (if (== (.playerindex (Variables|/Game/Blueprints/BP_GameInstance.BP_GameInstance_C|GetSettings _asbp_game_instance)) 0)
      (for _array_element (Collision|GetOverlappingActors (Variables|Default|GetAttackRadius) "/Game/Blueprints/Warrior_Character/BP_Warrior_Char.BP_Warrior_Char_C" :!class /Script/Engine.PrimitiveComponent)
        (Game|Damage|ApplyDamage _array_element (Variables|Default|GetAttackDamage) 0 0))
      (else
        (bind _asbp_game_instance_2 (Utilities|Casting|CastToBP_GameInstance (Game|GetGameInstance)))
        (if (== (.playerindex (Variables|/Game/Blueprints/BP_GameInstance.BP_GameInstance_C|GetSettings _asbp_game_instance_2)) 1)
          (for _array_element_2 (Collision|GetOverlappingActors (Variables|Default|GetAttackRadius) "/Game/Blueprints/Fireball_Character/BP_Fireball_Char.BP_Fireball_Char_C" :!class /Script/Engine.PrimitiveComponent)
            (Game|Damage|ApplyDamage _array_element_2 (Variables|Default|GetAttackDamage) 0 0))
          (else
            (bind _asbp_game_instance_3 (Utilities|Casting|CastToBP_GameInstance (Game|GetGameInstance)))
            (if (== (.playerindex (Variables|/Game/Blueprints/BP_GameInstance.BP_GameInstance_C|GetSettings _asbp_game_instance_3)) 2)
              (for _array_element_3 (Collision|GetOverlappingActors (Variables|Default|GetAttackRadius) "/Game/Blueprints/Iceball_Character/BP_Iceball_Char.BP_Iceball_Char_C" :!class /Script/Engine.PrimitiveComponent)
                (Game|Damage|ApplyDamage _array_element_3 (Variables|Default|GetAttackDamage) 0 0)))))))))

(event EventBeginPlay
  ;[0.7044 1 0.954] Event BeginPlay - Loops the damage control event and runs the behavior tree of the AI.
  (Utilities|Time|SetTimerbyFunctionName 0 "DamageControl" 0.1 true)
  (AI|RunBehaviorTree (AI|GetAIController self) "/Game/Blueprints/Carboard_Enemy/BT_Enemy.BT_Enemy"))

(event EventCharacterDied
  ;[1 0 0.9184] When the enemy dies, death animation works and the enemy destroys in 5 seconds.
  (Class|COABaseCharacter|ChangeAnimState "CAS_DEATH")
  (AI|Logic|StopLogic (Variables|/Script/AIModule.AIController|GetBrainComponent (AI|GetAIController (Pawn|GetController))) "Dead")
  (Collision|SetCollisionResponsetoChannel (Variables|Default|GetCapsuleComponent) "ECC_Pawn" "ECR_Ignore")
  (Utilities|FlowControl|Delay 5.0)
  (Actor|DestroyActor self))

(fn ConstructionScript)

(fn ModifyDamage
  (params (damage :type Float%20%28single-precision%29))
  ;[1 1 1] Decreases the enemy's health by the amount of damage taken plays the character's damage sound.
  (Variables|Default|SetisDamage? true)
  (Audio|PlaySound2D "/Game/Assets/Audio/Enemy/dying_cue.dying_cue" 1.5 1.0 0.0 0 0)
  (return damage))

(fn UpdateWalkSpeed
  (params (NewWalkSpeed :type Float%20%28single-precision%29))
  ;[1 1 1] Changes the Enemy's walking speed.
  (Variables|/Script/Engine.CharacterMovementComponent|SetMaxWalkSpeed (Variables|Character|GetCharacterMovement) NewWalkSpeed))