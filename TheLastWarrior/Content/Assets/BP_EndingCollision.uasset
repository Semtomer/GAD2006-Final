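; BP_EndingCollision is an end-of-game trigger that fires the win condition when a player character enters the house.
; On overlap, it compares the other actor to the first found instance of the Warrior, Fireball and Iceball character classes.
; A match sets IsEnd, then a DoOnce plays the Win sound, waits briefly and quits the game.
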(event Collision|EventActorBeginOverlap
  (params (OtherActor :type Actor%20Object%20Reference))
  ;[1 1 1] The game is over when the character enters the house. The win condition works and the winning sound plays. Exits after 5 seconds of the game.
  (Variables|Default|SetOverlappedActor OtherActor)
  (bind _outactors (Actor|GetAllActorsOfClass "/Game/Blueprints/Warrior_Character/BP_Warrior_Char.BP_Warrior_Char_C"))
  (bind _outactors_2 (Actor|GetAllActorsOfClass "/Game/Blueprints/Fireball_Character/BP_Fireball_Char.BP_Fireball_Char_C"))
  (bind _outactors_3 (Actor|GetAllActorsOfClass "/Game/Blueprints/Iceball_Character/BP_Iceball_Char.BP_Iceball_Char_C"))
  (if (Math|Boolean|ORBoolean (== (Utilities|Array|Get(acopy) _outactors_3) (Variables|Default|GetOverlappedActor)) (== (Utilities|Array|Get(acopy) _outactors_2) (Variables|Default|GetOverlappedActor)) (== (Utilities|Array|Get(acopy) _outactors) (Variables|Default|GetOverlappedActor)))
    (Variables|Default|SetisEnd? true)
    (Utilities|FlowControl|DoOnce false
      (:Completed
        (Audio|PlaySound2D "/Game/Assets/Audio/win.win" 1.0 1.0 0.0 0 0)
        (Utilities|FlowControl|Delay 5.0)
        (Game|QuitGame 0 "Quit" false)))))

(fn ConstructionScript)